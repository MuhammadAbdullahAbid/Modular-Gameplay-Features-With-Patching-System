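; Game mode that drives content patching at startup, showing a loading screen before travelling to TestChunkMap.
; On BeginPlay it binds to the MGF game instance's patch-ready event, which on success starts patching, then creates the loading widget and unbinds.
; Tick writes download percentage to the widget every frame, without checking the in-progress flag, and opens the map after a short delay once download and mount both complete.
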(event Custom|OnPatchReady
  (params (Succeeded :type Boolean))
  (if Succeeded
    (bind _returnvalue (Class|MGFGameInstance|PatchGame (Variables|Default|GetAs%20BP%20MGFGame%20Instance)))
    (Development|PrintString (Utilities|String|ToString(Boolean) _returnvalue))
    (bind _output_get (Variables|Default|SetIsPatchingInProgress _returnvalue))
    (if _output_get
      (bind _returnvalue_2 (UserInterface|CreateWidget "/Game/WBP_Loading.WBP_Loading_C"))
      (bind _output_get_2 (Variables|Default|SetWBP_Loading _returnvalue_2))
      (UserInterface|Viewport|AddtoViewport _output_get_2 0)
      (EventDispatchers|UnbindallEventsfromOnPatchReady (Variables|Default|GetAs%20BP%20MGFGame%20Instance)))))

(event EventBeginPlay
  (Development|PrintString "Casitng")
  (bind _asbp_mgfgame_instance (Utilities|Casting|CastToBP_MGFGameInstance (Game|GetGameInstance))
    (:then
      (bind _output_get (Variables|Default|SetAs%20BP%20MGFGame%20Instance _asbp_mgfgame_instance))
      (EventDispatchers|BindEventtoOnPatchReady _output_get (delegate Custom|OnPatchReady)))
    (:CastFailed
      (Development|PrintString "Cast Failed"))))

(event EventTick
  (params (DeltaSeconds :type Float%20%28single-precision%29))
  (bind _as_bp_mgfgame_instance (Variables|Default|GetAs%20BP%20MGFGame%20Instance))
  (bind (_filesdownloaded _totalfilestodownload _downloadpercent _chunksmounted _totalchunkstomount _mountpercent) (Class|MGFGameInstance|GetLoadingProgress _as_bp_mgfgame_instance))
  (Rendering|Components|TextRender|SetText (Variables|/Game/WBP_Loading.WBP_Loading_C|GetLoading (Variables|Default|GetWBP_Loading)) "Loading Patch: ")
  (Rendering|Components|TextRender|SetText (Variables|/Game/WBP_Loading.WBP_Loading_C|GetPercentage (Variables|Default|GetWBP_Loading)) (Utilities|Text|ToText(String) (Utilities|String|Append (Utilities|String|ToString(Float) (* _downloadpercent 1e+02)) " %")))
  (if (and (>= _downloadpercent 1.0) (>= _mountpercent 1.0))
    (Utilities|FlowControl|Delay 1.0)
    (Game|OpenLevel(byName) "TestChunkMap")))

(fn ConstructionScript)